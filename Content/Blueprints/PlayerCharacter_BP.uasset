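; Player character for a telefrag deathmatch that kills other players by overlapping them while teleporting.
; Beacon events spawn or destroy a teleport marker; teleporting disables capsule collision and uses custom movement to glide toward it until close.
; Teleport start and stop swap dynamic post-process materials and notify the player controller.
; Any damage increments the instigator's score, has the victim's controller handle the kill, and destroys the character.
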(event `InputAxis|MoveForward`
  (params (AxisValue :type "Float (single-precision)"))
  ;[1 1 1] Movement
  (`self.AddMovementInput` (`self.GetActorForwardVector`) AxisValue))

(event `Destroy beacon`
  ;[1 1 1] Server-Destroy Beacon
  (`self.K2_DestroyActor` (`self.Beacon`)))

(event `Spawn Beacon`
  ;[1 1 1] Server-Spawn Beacon
  (bind _returnvalue (`|SpawnActorFromClass` "/Game/Blueprints/TeleBeacon_BP.TeleBeacon_BP_C" (`self.GetTransform`) true))
  (set `self.Beacon` _returnvalue))

(event `InputAxis|MoveRight`
  (params (AxisValue :type "Float (single-precision)"))
  ;[1 1 1] Movement
  (`self.AddMovementInput` (`self.GetActorRightVector`) AxisValue))

(event `Stop Teleport`
  ;[1 1 1] Server-Stop Teleport
  (`self.K2_DestroyActor` (`self.Beacon`))
  (`CharacterMovementComponent.SetMovementMode` (`self.CharacterMovement`) "MOVE_Falling" 1)
  (`PrimitiveComponent.SetCollisionEnabled` (`self.CapsuleComponent`) "QueryAndPhysics")
  (set `self.IsTeleporting` false)
  (`KismetArrayLibrary.Array_Set` (`self.Get Post Effects Array` (`self.Post Process`)) 0 (`self.No Effect Material`) true)
  (bind _astelefraggerplayercontroller_bp_c (cast `/Game/Blueprints/TelefraggerPlayerController_BP` (`self.GetController`)))
  (`/Game/Blueprints/TelefraggerPlayerController_BP.Stop Teleport` _astelefraggerplayercontroller_bp_c))

(event `InputAxis|Horizontal`
  (params (AxisValue :type "Float (single-precision)"))
  ;[1 1 1] Mouse Axis
  (`self.AddControllerYawInput` AxisValue))

(event `InputAxis|Vertical`
  (params (AxisValue :type "Float (single-precision)"))
  ;[1 1 1] Mouse Axis
  (`self.AddControllerPitchInput` AxisValue))

(event `self.K2_UpdateCustomMovement`
  (params (DeltaTime :type "Float (single-precision)"))
  (bind _returnvalue (`self.K2_GetActorLocation` (`self.Beacon`)))
  (bind _returnvalue_2 (`SceneComponent.K2_GetComponentLocation` (`self.Bottom`)))
  ;[1 1 1] Teleport Movement
  (if (< (`self.Vector Distance` _returnvalue_2 _returnvalue) 50.0)
    (`self.Stop Teleport`)
    (else
      (`MovementComponent.K2_MoveUpdatedComponent` :`self` (`self.CharacterMovement`) :`Delta` (* (`KismetMathLibrary.Normal` (- _returnvalue _returnvalue_2)) (* DeltaTime (`self.TeleportSpeed`)))))))

(event `Start Teleport`
  ;[1 1 1] Server-Start Teleport
  (set `self.IsTeleporting` true)
  (`PrimitiveComponent.SetCollisionEnabled` (`self.CapsuleComponent`) "NoCollision")
  (`CharacterMovementComponent.SetMovementMode` (`self.CharacterMovement`) "MOVE_Custom" 1)
  (`KismetArrayLibrary.Array_Set` (`self.Get Post Effects Array` (`self.Post Process`)) 0 (`self.TelePostMaterial`) true)
  (bind _astelefraggerplayercontroller_bp_c (cast `/Game/Blueprints/TelefraggerPlayerController_BP` (`self.GetController`)))
  (`/Game/Blueprints/TelefraggerPlayerController_BP.Start Teleport` _astelefraggerplayercontroller_bp_c))

(event `InputAxis|HorizontalRate`
  (params (AxisValue :type "Float (single-precision)"))
  ;[1 1 1] Not Tested Controler Axis
  (`self.AddControllerYawInput` (* AxisValue (`self.BaseTurnRate`) (`GameplayStatics.GetWorldDeltaSeconds`))))

(event `InputAxis|VerticalRate`
  (params (AxisValue :type "Float (single-precision)"))
  ;[1 1 1] Not Tested Controler Axis
  (`self.AddControllerPitchInput` (* AxisValue (`self.BaseTurnRate`) (`GameplayStatics.GetWorldDeltaSeconds`))))

(event `self.ReceiveActorBeginOverlap`
  (params (OtherActor :type "Actor Object Reference"))
  (bind _asplayercharacter_bp_c (cast `/Game/Blueprints/PlayerCharacter_BP` OtherActor))
  (if (`/Game/Blueprints/PlayerCharacter_BP.IsTeleporting` _asplayercharacter_bp_c)
    _
    (elif (`self.IsTeleporting`)
      (`GameplayStatics.ApplyDamage` OtherActor 1.0 (`self.GetController` self) self))))

(event `self.ReceiveAnyDamage`
  (params (Damage :type "Float (single-precision)") (DamageType :type "DamageType Object Reference") (InstigatedBy :type "Controller Object Reference") (DamageCauser :type "Actor Object Reference"))
  (bind _asdeathmatchplayerstate (cast `DeathmatchPlayerState` (`Controller.PlayerState` InstigatedBy)))
  (`DeathmatchPlayerState.IncrementScore` _asdeathmatchplayerstate)
  (bind _astelefraggerplayercontroller_bp_c (cast `/Game/Blueprints/TelefraggerPlayerController_BP` (`self.GetController`)))
  (`/Game/Blueprints/TelefraggerPlayerController_BP.Kill` _astelefraggerplayercontroller_bp_c (`self.GetTransform`))
  (`self.K2_DestroyActor`))

(fn `UserConstructionScript`
  (bind _returnvalue (`KismetMaterialLibrary.CreateDynamicMaterialInstance` "/Game/Materials/Post/TeleportPostEffect.TeleportPostEffect"))
  (set `self.TelePostMaterial` _returnvalue)
  (`MaterialInstanceDynamic.SetScalarParameterValue` (`self.TelePostMaterial`) "Fraction" 0.5)
  (bind _returnvalue_2 (`KismetMaterialLibrary.CreateDynamicMaterialInstance` "/Game/Materials/Post/NoEffectPostEffect.NoEffectPostEffect"))
  (set `self.No Effect Material` _returnvalue_2))
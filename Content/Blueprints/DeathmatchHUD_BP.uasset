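; Deathmatch HUD that shows scores and manages the chat entry widget.
; DrawHUD draws the player's score and a list of every GameState PlayerArray name and rounded score, stacked in evenly spaced rows.
; EnableChatMode opens a single modal ChatWidget_BP with cursor and gives it a reference back to the HUD.
; DisableChatMode clears the chat state and widget reference, then passes the message to SendChat.
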(event Custom|EnableChatMode
  (if (not (Variables|Default|GetChatMode))
    (bind _returnvalue (Class|WidgetBlueprintLibrary|Create "/Game/Widgets/ChatWidget_BP.ChatWidget_BP_C" (Game|Player|GetOwningPlayerController)))
    (UserInterface|Viewport|AddtoViewport _returnvalue false true true)
    (Variables|Default|SetChatWidget _returnvalue)
    (bind _aschatwidget_bp_c (Utilities|Casting|CastToChatWidget_BP _returnvalue))
    (Variables|/Game/Widgets/ChatWidget_BP.ChatWidget_BP_C|SetHudBackRef _aschatwidget_bp_c self)
    (Variables|Default|SetChatMode true)))

(event Custom|DisableChatMode
  (params (Message :type String))
  (Variables|Default|SetChatMode false)
  (Variables|Default|SetChatWidget 0)
  (Class|DeathmatchHUD|SendChat Message))

(event EventDrawHUD
  (params (SizeX :type Integer) (SizeY :type Integer))
  (HUD|DrawText (Utilities|String|Append "Score: " (Utilities|String|ToString(Integer) (Class|DeathmatchHUD|GetPlayerScore))) "(R=1.000000,G=1.000000,B=1.000000,A=1.000000)" 0.0 0.0 "/Engine/EngineFonts/RobotoDistanceField.RobotoDistanceField" 2.0 false)
  (for (_array_element _array_index) (Variables|/Script/Engine.GameState|GetPlayerArray (Game|GetGameState))
    (HUD|DrawText (Utilities|String|Append (Utilities|String|Append (Variables|/Script/Engine.PlayerState|GetPlayerName _array_element) ": ") (Utilities|String|ToString(Integer) (Math|Float|Round (Variables|/Script/Engine.PlayerState|GetScore _array_element)))) "(R=1.000000,G=1.000000,B=1.000000,A=1.000000)" 0.0 (|48+(x*20) (Math|Conversions|ToFloat(Integer) _array_index)) "/Engine/EngineFonts/RobotoDistanceField.RobotoDistanceField" 1.0 false)))

(fn ConstructionScript)